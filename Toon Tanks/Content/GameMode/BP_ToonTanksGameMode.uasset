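; Game mode for Toon Tanks that shows the start and end screens of a match.
; StartGame adds the start-game widget to the viewport.
; GameOver shows the mouse cursor, switches to UI-only input and adds the end-game widget, setting its text to a win or lose message based on the WonGame flag.
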(event `self.StartGame`
  (bind _returnvalue (`|CreateWidget` "/Game/Blueprints/Widgets/WBP_StartGameWidget.WBP_StartGameWidget_C"))
  (`UserWidget.AddToViewport` _returnvalue 0))

(event `self.GameOver`
  (params (bWonGame :type Boolean))
  (bind _returnvalue (`GameplayStatics.GetPlayerController` 0))
  (set `PlayerController.bShowMouseCursor` true _returnvalue)
  (`WidgetBlueprintLibrary.SetInputMode_UIOnlyEx` _returnvalue null)
  (bind _returnvalue_2 (`|CreateWidget` "/Game/Blueprints/Widgets/WBP_EndGameWidget.WBP_EndGameWidget_C"))
  (`UserWidget.AddToViewport` _returnvalue_2 0)
  (if bWonGame
    (set `self.EndGameString` "You Win!")
    (else
      (set `self.EndGameString` "You Lose :(")))
  (`TextBlock.SetText` (`/Game/Blueprints/Widgets/WBP_EndGameWidget.DisplayText` _returnvalue_2) (`KismetTextLibrary.Conv_StringToText` (`self.EndGameString`))))

(fn `UserConstructionScript`)